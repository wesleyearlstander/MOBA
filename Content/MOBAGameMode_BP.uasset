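; MOBA game mode that builds per-team creep lane paths and runs the minion wave timer.
; On BeginPlay it counts CreepWaypoint_BP actors per lane, then sorts them by Order into three lane arrays per team, with Team 2's reversed.
; After a short delay it calls SpawnMinionWave on a looping timer, though that event is empty here.
; GetWaypointsForTeam returns the path for a given team and lane.
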(event `self.ReceiveBeginPlay`
  (bind _waypointcounts (`self.WayPointCounts`))
  (bind _waypointcounts_2 (`self.WayPointCounts`))
  (`|ExecutionSequence`
    (:`then_0`
      (bind _outactors (`GameplayStatics.GetAllActorsOfClass` "/Game/CreepWaypoint_BP.CreepWaypoint_BP_C"))
      (`KismetArrayLibrary.Array_Clear` _waypointcounts)
      (`KismetArrayLibrary.Array_Resize` _waypointcounts 3)
      (for _array_element _outactors
        (bind _returnvalue (`KismetMathLibrary.Conv_ByteToInt` (`CreepWaypoint.lane` _array_element)))
        (bind _result (`/Engine/EditorBlueprintResources/StandardMacros.IncrementInt` (`|GetArrayItem` _waypointcounts_2 _returnvalue))
          (:`  `
            (`KismetArrayLibrary.Array_Set` _waypointcounts_2 _returnvalue _result))))
      (for _array_element_2 _outactors
        (bind _returnvalue_2 (`KismetMathLibrary.Conv_ByteToInt` (`CreepWaypoint.lane` _array_element_2)))
        (switch `int` _returnvalue_2
          (:`0`
            (bind _order (`CreepWaypoint.order` _array_element_2))
            (`KismetArrayLibrary.Array_Set` (`self.Team1LaneTop`) _order _array_element_2 true)
            (bind _returnvalue_3 (- (- (`|GetArrayItem` (`self.WayPointCounts`) _returnvalue_2) 1) _order))
            (`KismetArrayLibrary.Array_Set` (`self.Team2LaneTop`) _returnvalue_3 _array_element_2 true))
          (:`1`
            (`KismetArrayLibrary.Array_Set` (`self.Team1LaneMiddle`) _order _array_element_2 true)
            (`KismetArrayLibrary.Array_Set` (`self.Team2LaneMiddle`) _returnvalue_3 _array_element_2 true))
          (:`2`
            (`KismetArrayLibrary.Array_Set` (`self.Team1LaneBottom`) _order _array_element_2 true)
            (`KismetArrayLibrary.Array_Set` (`self.Team2LaneBottom`) _returnvalue_3 _array_element_2 true)))))
    (:`then_1`
      (`KismetSystemLibrary.Delay` 1.0)
      (`self.Spawn Minion Wave`)
      (`KismetSystemLibrary.K2_SetTimerDelegate` (delegate `Spawn Minion Wave`) (`self.WaveRespawnTimer`) true))))

(event `Spawn Minion Wave`)

(fn `Get Waypoints for team`
  (params (Team :type "Team Enum" :default "Red") (Lane :type "Lane Enum" :default "Top"))
  (returns (Waypoints :type "Array of Actor Object Reference"))
  (switch `Team` Team
    (:`Red`
      (switch `Lane` Lane
        (:`Top`
          (return (`self.Team1LaneTop`)))
        (:`Middle`
          (return (`self.Team1LaneMiddle`)))
        (:`Bottom`
          (return (`self.Team1LaneBottom`)))))
    (:`Blue`
      (switch `Lane` Lane
        (:`Top`
          (return (`self.Team2LaneTop`)))
        (:`Middle`
          (return (`self.Team2LaneMiddle`)))
        (:`Bottom`
          (return (`self.Team2LaneBottom`)))))))

(fn `UserConstructionScript`)