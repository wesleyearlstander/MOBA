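; AI controller for creeps, driving waypoint movement and enemy detection through a behavior tree.
; On possession it waits briefly, runs CreepBehaviourTree and seeds the blackboard with the first waypoint as target, a moving state and attack range.
; AI perception updates on other creeps compare teams, making a sensed enemy the target.
; Any other creep update, including lost sight or a same-team creep, clears the can-see and attacking flags.
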(event `self.ReceivePossess`
  (params (PossessedPawn :type "Pawn Object Reference"))
  (bind _returnvalue (`AIBlueprintHelperLibrary.GetBlackboard` (`AIBlueprintHelperLibrary.GetAIController` PossessedPawn)))
  (`KismetSystemLibrary.Delay` 1.0)
  (`self.RunBehaviorTree` "/Game/Creep/Creep_AI/CreepBehaviourTree.CreepBehaviourTree")
  (`BlackboardComponent.SetValueAsInt` _returnvalue (`self.CurrentWaypointKey`) 0)
  (`BlackboardComponent.SetValueAsObject` _returnvalue (`self.TargetActorKey`) (`|GetArrayItem` (`self.Waypoints`)))
  (`BlackboardComponent.SetValueAsBool` _returnvalue (`self.MovingKey`) true)
  (`BlackboardComponent.SetValueAsInt` _returnvalue (`self.AttackRange`) 50))

(event `self.AIPerception.OnTargetPerceptionUpdated`
  (params (Actor :type "Actor Object Reference") (Stimulus :type "AIStimulus Structure"))
  (bind _returnvalue (`self.K2_GetPawn`))
  (bind _returnvalue_2 (`AIBlueprintHelperLibrary.GetBlackboard` _returnvalue))
  (bind _ascreep_bp (cast `/Game/Creep/Creep_BP` Actor))
  (bind _ascreep_bp_2 (cast `/Game/Creep/Creep_BP` _returnvalue))
  (bind _returnvalue_3 (and (`.bSuccessfullySensed` (break `AIStimulus` Stimulus)) (!= (`CreepCharacter.Team` _ascreep_bp_2) (`CreepCharacter.Team` _ascreep_bp))))
  (`BlackboardComponent.SetValueAsBool` _returnvalue_2 (`self.CanSeeCreepKey`) _returnvalue_3)
  (if _returnvalue_3
    (`BlackboardComponent.SetValueAsObject` _returnvalue_2 (`self.TargetActorKey`) _ascreep_bp)
    (else
      (`BlackboardComponent.SetValueAsBool` _returnvalue_2 (`self.AttackingKey`) false))))

(fn `UserConstructionScript`)