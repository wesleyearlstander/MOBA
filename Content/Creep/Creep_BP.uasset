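; Creep actor Blueprint with a world-space health bar widget that always faces the player's camera.
; On BeginPlay it casts the widget component's object to CreepHealthBar and hands it a reference to itself.
; Each tick, HealthBarBillboard rotates the widget component to point opposite the first player's camera manager forward vector, so it stays parallel to the view.
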(event `self.ReceiveBeginPlay`
  (bind _ascreep_health_bar (cast `/Game/Creep/CreepHealthBar` (`WidgetComponent.GetUserWidgetObject` (`self.HealthBarUI`))))
  (set `/Game/Creep/CreepHealthBar.Creep` self _ascreep_health_bar))

(event `self.ReceiveTick`
  (params (DeltaSeconds :type "Float (single-precision)"))
  (`self.HealthBarBillboard`))

(fn `UserConstructionScript`)